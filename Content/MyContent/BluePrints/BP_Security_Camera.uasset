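; BP_Security_Camera is a stealth-level security camera that catches the first-person player and restarts the map.
; A self-repeating, delayed loop alternates CurrentRotation between start and end through a FlipFlop, though its MoveComponentTo always targets EndRotation.
; Every tick, a debug-drawn pawn line trace runs forward from SMLineTrace up to DetectDistance.
; Hitting the cached player prints "Caught", disables input, then reloads StealthMap after a delay.
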(event Custom|Move%20Camera
  (bind _endrotation (Variables|Default|GetEndRotation))
  (Utilities|FlowControl|FlipFlop
    (:A
      (Variables|Default|SetCurrentRotation (Variables|Default|GetStartRotation)))
    (:B
      (Variables|Default|SetCurrentRotation (Variables|Default|GetEndRotation))))
  (Components|MoveComponentTo (Variables|Default|GetSM_Camera) "0, 0, 0" (Math|Rotator|MakeRotator (.x _endrotation) (.y _endrotation) (.z _endrotation)) false false (Variables|Default|GetSpeed) false)
  (Utilities|FlowControl|Delay (Variables|Default|GetDelay))
  (CallFunction|MoveCamera))

(event Custom|Detect
  (bind _bp_first_person_character (Variables|Default|GetBP%20First%20Person%20Character))
  (bind _sm_line_trace (Variables|Default|GetSM_Line_Trace))
  (bind _returnvalue (Transformation|GetWorldLocation _sm_line_trace))
  ;[0.15 0.15 0.15 0.5] Check for player in sight
  (bind _outhit (Collision|LineTraceForObjects _returnvalue (+ _returnvalue (* (Math|Vector|GetForwardVector (Transformation|GetWorldRotation _sm_line_trace)) (Variables|Default|GetDetectDistance))) (Utilities|Array|MakeArray "ObjectTypeQuery3") false 0 "ForOneFrame"))
  (if (== (.HitActor (Collision|BreakHitResult _outhit)) _bp_first_person_character)
    ;[0.15 0.15 0.15 0.5] On Caught
    (Development|PrintString "Caught")
    (Input|DisableInput _bp_first_person_character (Game|GetPlayerController 0))
    (Utilities|FlowControl|Delay (Variables|Default|GetReloadDelay))
    (Game|OpenLevel(byName) "StealthMap")))

(event EventBeginPlay
  ;[0.15 0.15 0.15 0.5] Get player character
  (bind _asbp_first_person_character (Utilities|Casting|CastToBP_FirstPersonCharacter (Game|GetPlayerCharacter 0)))
  (Variables|Default|SetBP%20First%20Person%20Character _asbp_first_person_character)
  (CallFunction|MoveCamera))

(event EventTick
  (params (DeltaSeconds :type Float%20%28single-precision%29))
  (CallFunction|Detect))

(fn ConstructionScript)