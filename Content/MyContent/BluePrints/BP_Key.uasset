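; BP_Key is a pickup key that appears once enough BP_Target actors are destroyed and grants the player HasKey.
; Tick polls the BP_Target count against a hard-coded threshold, using an array Add's returned index, to toggle the key's visibility and collision.
; A DoOnce plays the appearance effect and sound.
; Player overlap while revealed sets the flag, plays the collect sound and destroys the key.
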(event OnComponentBeginOverlap(Collision)
  (params (OverlappedComponent :type Primitive%20Component%20Object%20Reference) (OtherActor :type Actor%20Object%20Reference) (OtherComp :type Primitive%20Component%20Object%20Reference) (OtherBodyIndex :type Integer) (bFromSweep :type Boolean) (SweepResult :type Hit%20Result%20Structure%20%28by%20ref%29))
  (bind _bp_first_person_character (Variables|Default|GetBP%20First%20Person%20Character))
  ;[0.15 0.15 0.15 0.5] Collision with player
  (if (and (== OtherActor _bp_first_person_character) (Variables|Default|GetAllTargetsDestroyed))
    (Variables|/Game/StarterContent/FirstPerson/Blueprints/BP_FirstPersonCharacter.BP_FirstPersonCharacter_C|SetHasKey _bp_first_person_character true)
    (Audio|PlaySoundatLocation "/Game/MyContent/Audio/MP3_Key_Collect.MP3_Key_Collect" (Transformation|GetActorLocation _bp_first_person_character) "0, 0, 0" 1.0 1.0 0.0 0 0 0 0)
    (Actor|DestroyActor)))

(event EventBeginPlay
  (bind _asbp_first_person_character (Utilities|Casting|CastToBP_FirstPersonCharacter (Game|GetPlayerCharacter 0)))
  (Variables|Default|SetBP%20First%20Person%20Character _asbp_first_person_character))

(event EventTick
  (params (DeltaSeconds :type Float%20%28single-precision%29))
  (bind _returnvalue (Transformation|GetActorLocation))
  ;[0.15 0.15 0.15 0.5] Visibility
  (bind _outactors (Actor|GetAllActorsOfClass "/Game/MyContent/BluePrints/BP_Target.BP_Target_C"))
  (bind _returnvalue_2 (Utilities|Array|Add _outactors 0))
  (bind _output_get (Variables|Default|SetAllTargetsDestroyed (<= _returnvalue_2 18)))
  (Rendering|SetVisibility (Variables|Default|GetSM_Key) _output_get false)
  (Collision|SetActorEnableCollision _output_get)
  ;[0.15 0.15 0.15 0.5] All Targets are Destroyed
  (if (Variables|Default|GetAllTargetsDestroyed)
    (Utilities|FlowControl|DoOnce false
      (:Completed
        (Niagara|SpawnSystematLocation "/Game/MyContent/FX/PE_Target_Hit.PE_Target_Hit" _returnvalue)
        (Audio|SpawnSoundatLocation "/Game/MyContent/Audio/MP3_Key_Appear.MP3_Key_Appear" _returnvalue "0, 0, 0" 1.0 1.0 0.0 0 0)))))

(fn ConstructionScript)