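; BP_Door is a key-locked door that swings open when the first-person player enters its collision area while holding a key.
; On BeginPlay it caches the player character and puts a dynamic material instance on the door light mesh.
; On overlap the light brightens, turning green and playing a Timeline that rotates the door if HasKey is set, or red otherwise.
; Leaving dims the light to yellow and reverses the Timeline.
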(event OnComponentBeginOverlap(Collision)
  (params (OverlappedComponent :type Primitive%20Component%20Object%20Reference) (OtherActor :type Actor%20Object%20Reference) (OtherComp :type Primitive%20Component%20Object%20Reference) (OtherBodyIndex :type Integer) (bFromSweep :type Boolean) (SweepResult :type Hit%20Result%20Structure%20%28by%20ref%29))
  (bind _dynamicmaterial (Variables|Default|GetDynamicMaterial))
  (bind _bp_first_person_character (Variables|Default|GetBP%20First%20Person%20Character))
  (if (== OtherActor _bp_first_person_character)
    (Rendering|Material|SetScalarParameterValue _dynamicmaterial "Intensity" 1e+02 :!class /Script/Engine.MaterialInstanceDynamic)
    (if (Variables|/Game/StarterContent/FirstPerson/Blueprints/BP_FirstPersonCharacter.BP_FirstPersonCharacter_C|GetHasKey _bp_first_person_character)
      (Rendering|Material|SetVectorParameterValue _dynamicmaterial "Colour" "(R=0.000000,G=1.000000,B=0.009535,A=1.000000)" :!class /Script/Engine.MaterialInstanceDynamic)
      (bind _alpha (Timeline|Timeline Play)
        (:Update
          (Transformation|SetRelativeRotation (Variables|Default|GetSM_Door) (Math|Rotator|Lerp(Rotator) "0, 0, 0" "0.000000,90.000000,0.000000" _alpha) false false)))
      (else
        (Rendering|Material|SetVectorParameterValue _dynamicmaterial "Colour" "(R=1.000000,G=0.000000,B=0.003028,A=1.000000)" :!class /Script/Engine.MaterialInstanceDynamic)))))

(event OnComponentEndOverlap(Collision)
  (params (OverlappedComponent :type Primitive%20Component%20Object%20Reference) (OtherActor :type Actor%20Object%20Reference) (OtherComp :type Primitive%20Component%20Object%20Reference) (OtherBodyIndex :type Integer))
  (bind _dynamicmaterial (Variables|Default|GetDynamicMaterial))
  (if (== OtherActor (Variables|Default|GetBP%20First%20Person%20Character))
    (Rendering|Material|SetScalarParameterValue _dynamicmaterial "Intensity" 1.0 :!class /Script/Engine.MaterialInstanceDynamic)
    (Rendering|Material|SetVectorParameterValue _dynamicmaterial "Colour" "(R=0.979442,G=1.000000,B=0.000000,A=1.000000)" :!class /Script/Engine.MaterialInstanceDynamic)
    (bind _alpha (Timeline|Timeline Reverse)
      (:Update
        (Transformation|SetRelativeRotation (Variables|Default|GetSM_Door) (Math|Rotator|Lerp(Rotator) "0, 0, 0" "0.000000,90.000000,0.000000" _alpha) false false)))))

(event EventBeginPlay
  (bind _asbp_first_person_character (Utilities|Casting|CastToBP_FirstPersonCharacter (Game|GetPlayerCharacter 0)))
  (Variables|Default|SetBP%20First%20Person%20Character _asbp_first_person_character)
  (bind _returnvalue (Rendering|Material|CreateDynamicMaterialInstance "/Game/MyContent/Materials/MI_Doorlight.MI_Doorlight" "None" "None" :!class /Script/Engine.KismetMaterialLibrary))
  (bind _output_get (Variables|Default|SetDynamicMaterial _returnvalue))
  (Rendering|Material|SetMaterial (Variables|Default|GetSM_DoorLight) 0 _output_get))

(fn ConstructionScript)