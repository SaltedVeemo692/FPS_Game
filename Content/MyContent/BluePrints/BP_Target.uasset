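; BP_Target is a moving, destructible target actor with two movement modes, applied every tick without delta-time scaling.
; Normal mode slides along Direction, which a looping timer reverses; Increment mode rotates by DirectionIncrement while stepping along a local offset from that rotator's right vector.
; Each hit destroys the other actor and decrements HitPoint, playing a small explosion sound, or spawning destroy FX and a big explosion before removing itself at zero.
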(event Custom|Event_Flip_Direction
  ;[0.15 0.15 0.15 0.5] Flip Direction
  (Variables|Default|SetDirection (* (Variables|Default|GetDirection) -1.0)))

(event EventBeginPlay
  ;[0.15 0.15 0.15 0.5] Flip Direction
  (switch Utilities|FlowControl|Switch|SwitchonE_TargetMovementType (Variables|Default|GetMovementType)
    (:NewEnumerator0
      (Utilities|Time|SetTimerbyEvent (delegate Custom|Event_Flip_Direction) (Variables|Default|GetMovementDuration) true))))

(event EventTick
  (params (DeltaSeconds :type Float%20%28single-precision%29))
  (bind _speed (Variables|Default|GetSpeed))
  (bind _directionincrement (Variables|Default|GetDirectionIncrement))
  ;[0.15 0.15 0.15 0.5] Target Movement
  (switch Utilities|FlowControl|Switch|SwitchonE_TargetMovementType (Variables|Default|GetMovementType)
    (:NewEnumerator0
      ;[0.15 0.15 0.15 0.5] Normal
      (Transformation|AddActorWorldOffset (* (Math|Vector|Normalize (Variables|Default|GetDirection)) _speed)))
    (:NewEnumerator1
      ;[0.15 0.15 0.15 0.5] Increment
      (Class|Actor|AddActorWorldRotation _directionincrement)
      (Transformation|AddActorLocalOffset (* (Math|Vector|Normalize (Math|Vector|GetRightVector _directionincrement)) _speed) false false))))

(event Collision|EventHit
  (params (MyComp :type Primitive%20Component%20Object%20Reference) (Other :type Actor%20Object%20Reference) (OtherComp :type Primitive%20Component%20Object%20Reference) (bSelfMoved :type Boolean) (HitLocation :type Vector :default "0, 0, 0") (HitNormal :type Vector :default "0, 0, 0") (NormalImpulse :type Vector :default "0, 0, 0") (Hit :type Hit%20Result%20Structure%20%28by%20ref%29))
  ;[0.15 0.15 0.15 0.5] Target Hit
  (Actor|DestroyActor Other)
  (Variables|Default|SetHitPoint (- (Variables|Default|GetHitPoint) 1))
  (if (<= (Variables|Default|GetHitPoint) 0)
    ;[0.15 0.15 0.15 0.5] On Destroy
    (Niagara|SpawnSystematLocation (Variables|Default|GetDestroyFX) HitLocation)
    (Audio|SpawnSoundatLocation "/Game/MyContent/Audio/MP3_Explosion_Big.MP3_Explosion_Big" HitLocation "0, 0, 0" 1.0 1.0 0.0 0 0)
    (Actor|DestroyActor)
    (else
      ;[0.15 0.15 0.15 0.5] On Hit
      (Audio|SpawnSoundatLocation "/Game/MyContent/Audio/MP3_Explosions_Small.MP3_Explosions_Small" HitLocation "0, 0, 0" 1.0 1.0 0.0 0 0))))

(fn ConstructionScript)