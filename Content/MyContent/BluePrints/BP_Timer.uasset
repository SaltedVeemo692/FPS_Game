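; BP_Timer is an actor that times how long the player takes until no BP_Target actors remain in the level.
; Begin and end overlap share one branch, which sets IsActive if it is false and otherwise switches State to Count.
; Tick runs the Standby, Count and Finish states, accumulating and printing elapsed time while polling GetAllActorsOfClass every counting frame, then finishing when none are found.
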(event Collision|EventActorBeginOverlap
  (params (OtherActor :type Actor%20Object%20Reference))
  ;[0.15 0.15 0.15 0.5] Player Touch Initiate Timer
  (if (Variables|Default|GetIsActive)
    (Variables|Default|SetState "NewEnumerator1")
    (else
      (Variables|Default|SetIsActive true))))

(event Collision|EventActorEndOverlap
  (params (OtherActor :type Actor%20Object%20Reference))
  ;[0.15 0.15 0.15 0.5] Player Touch Initiate Timer
  (if (Variables|Default|GetIsActive)
    (Variables|Default|SetState "NewEnumerator1")
    (else
      (Variables|Default|SetIsActive true))))

(event EventTick
  (params (DeltaSeconds :type Float%20%28single-precision%29))
  ;[0.15 0.15 0.15 0.5] Check State
  (switch Utilities|FlowControl|Switch|SwitchonE_Timer_States (Variables|Default|GetState)
    (:NewEnumerator0
      ;[0.15 0.15 0.15 0.5] Standby
      (Variables|Default|SetTimeElapsed 0.0))
    (:NewEnumerator1
      ;[0.15 0.15 0.15 0.5] Count
      (bind _output_get (Variables|Default|SetTimeElapsed (+ (Variables|Default|GetTimeElapsed) DeltaSeconds)))
      ;[0.15 0.15 0.15 0.5] Check existing targets
      (bind _outactors (Actor|GetAllActorsOfClass "/Game/MyContent/BluePrints/BP_Target.BP_Target_C"))
      (if (<= (Utilities|Array|Length _outactors) 0)
        ;[0.15 0.15 0.15 0.5] All targets are gone
        (Variables|Default|SetState "NewEnumerator2")
        (Development|PrintString "Finish")
        (else
          ;[0.15 0.15 0.15 0.5] Targets still exist
          (Development|PrintString (Utilities|String|ToString(Float) _output_get)))))
    (:NewEnumerator2
      ;[0.15 0.15 0.15 0.5] Finish
      (Development|PrintString "FINISH"))))

(fn ConstructionScript)