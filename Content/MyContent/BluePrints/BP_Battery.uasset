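; BP_Battery is a battery pickup that adds to the first-person player's battery count.
; On BeginPlay it caches the player's BP_FirstPersonCharacter.
; When that character overlaps its Collision component while below BatteryCapacityMax, it increments BatteriesHeld, prints the count and a message, then destroys itself.
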(event OnComponentBeginOverlap(Collision)
  (params (OverlappedComponent :type Primitive%20Component%20Object%20Reference) (OtherActor :type Actor%20Object%20Reference) (OtherComp :type Primitive%20Component%20Object%20Reference) (OtherBodyIndex :type Integer) (bFromSweep :type Boolean) (SweepResult :type Hit%20Result%20Structure%20%28by%20ref%29))
  (bind _bp_first_person_character (Variables|Default|GetBP%20First%20Person%20Character))
  (bind _bp_first_person_character_2 (Variables|Default|GetBP%20First%20Person%20Character))
  ;[0.15 0.15 0.15 0.5] On pickup
  (if (and (== OtherActor _bp_first_person_character) (< (Variables|/Game/StarterContent/FirstPerson/Blueprints/BP_FirstPersonCharacter.BP_FirstPersonCharacter_C|GetBatteriesHeld _bp_first_person_character) (Variables|/Game/StarterContent/FirstPerson/Blueprints/BP_FirstPersonCharacter.BP_FirstPersonCharacter_C|GetBatteryCapacityMax _bp_first_person_character)))
    (bind _output_get (Variables|/Game/StarterContent/FirstPerson/Blueprints/BP_FirstPersonCharacter.BP_FirstPersonCharacter_C|SetBatteriesHeld _bp_first_person_character_2 (+ (Variables|/Game/StarterContent/FirstPerson/Blueprints/BP_FirstPersonCharacter.BP_FirstPersonCharacter_C|GetBatteriesHeld _bp_first_person_character_2) 1)))
    (Development|PrintString (Utilities|String|ToString(Integer) _output_get))
    (Development|PrintString "Get Battery!")
    (Actor|DestroyActor)))

(event EventBeginPlay
  ;[0.15 0.15 0.15 0.5] Get Player
  (bind _asbp_first_person_character (Utilities|Casting|CastToBP_FirstPersonCharacter (Game|GetPlayerCharacter 0)))
  (Variables|Default|SetBP%20First%20Person%20Character _asbp_first_person_character))

(fn ConstructionScript)