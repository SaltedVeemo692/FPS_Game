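; Pressure plate that destroys a linked door once every BP_Target in its check volume is gone.
; On BeginPlay it links the first overlapping BP_Door, or any overlapping actor as fallback, and gives its light a dynamic material.
; Tick polls for remaining targets, coloring the light red when locked and yellow when ready.
; Player overlap or a collision hit then latches it, glowing green and removing the door.
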(event OnComponentHit(Collision)
  (params (HitComponent :type Primitive%20Component%20Object%20Reference) (OtherActor :type Actor%20Object%20Reference) (OtherComp :type Primitive%20Component%20Object%20Reference) (NormalImpulse :type Vector :default "0, 0, 0") (Hit :type Hit%20Result%20Structure%20%28by%20ref%29))
  (bind _dynamic_material (Variables|Default|GetDynamic%20Material))
  ;[0.15 0.15 0.15 0.5] Check if shot or stepped
  (if (Variables|Default|GetCanActivate)
    ;[0.15 0.15 0.15 0.5] Activate Plate
    (Rendering|Material|SetScalarParameterValue _dynamic_material "Intensity" 2e+02 :!class /Script/Engine.MaterialInstanceDynamic)
    (Rendering|Material|SetVectorParameterValue _dynamic_material "Colour" "(R=0.000000,G=1.000000,B=0.000000,A=1.000000)" :!class /Script/Engine.MaterialInstanceDynamic)
    (Variables|Default|SetActivated true)
    ;[0.15 0.15 0.15 0.5] Destroy door
    (bind _door (Variables|Default|GetDoor)
      (:then
        (Actor|DestroyActor _door)
        (Variables|Default|SetCanActivate true)
        (Development|PrintString "Door Cleared"))
      (:else))))

(event EventBeginPlay
  (bind _c_door (Variables|Default|GetC_Door))
  ;[0.15 0.15 0.15 0.5] Initiate
  ;;[0.15 0.15 0.15 0.5] Get player
  (bind _asbp_first_person_character (Utilities|Casting|CastToBP_FirstPersonCharacter (Game|GetPlayerCharacter 0)))
  (Variables|Default|SetBP%20First%20Person%20Character _asbp_first_person_character)
  ;;[0.15 0.15 0.15 0.5] Get Door
  (bind _overlappingactors (Collision|GetOverlappingActors _c_door "/Game/MyContent/BluePrints/BP_Door.BP_Door_C" :!class /Script/Engine.PrimitiveComponent))
  (if (> (Utilities|Array|Length _overlappingactors) 0)
    ;;[0.15 0.15 0.15 0.5] If Door in bound
    (bind _asbp_door (Utilities|Casting|CastToBP_Door (Utilities|Array|Get(acopy) _overlappingactors)))
    (Variables|Default|SetDoor _asbp_door)
    ;;[0.15 0.15 0.15 0.5] Create Dynamic Material
    (bind _returnvalue (Rendering|Material|CreateDynamicMaterialInstance "/Game/MyContent/Materials/MI_Doorlight.MI_Doorlight" "None" "None" :!class /Script/Engine.KismetMaterialLibrary :!label _label))
    (bind _output_get (Variables|Default|SetDynamic%20Material _returnvalue))
    (Rendering|Material|SetMaterial (Variables|Default|GetSM_Light) 0 _output_get)
    (else
      ;;[0.15 0.15 0.15 0.5] If no doors
      (bind _overlappingactors_2 (Collision|GetOverlappingActors _c_door 0 :!class /Script/Engine.PrimitiveComponent))
      (if (> (Utilities|Array|Length _overlappingactors_2) 0)
        (Variables|Default|SetDoor (Utilities|Array|Get(acopy) _overlappingactors_2))
        (goto _label)
        (else
          (Development|PrintString "[WARNING] DOOR / OBJECT NOT DETECTED"))))))

(event EventTick
  (params (DeltaSeconds :type Float%20%28single-precision%29))
  (bind _dynamic_material (Variables|Default|GetDynamic%20Material))
  ;[0.15 0.15 0.15 0.5] Check Any Targets left
  (if (<= (Utilities|Array|Length (Collision|GetOverlappingActors (Variables|Default|GetC_CheckTargets) "/Game/MyContent/BluePrints/BP_Target.BP_Target_C" :!class /Script/Engine.PrimitiveComponent)) 0)
    ;[0.15 0.15 0.15 0.5] can activate
    (Rendering|Material|SetVectorParameterValue (Variables|Default|GetDynamic%20Material) "Colour" "(R=1.000000,G=0.931079,B=0.000000,A=1.000000)" :!class /Script/Engine.MaterialInstanceDynamic)
    (Variables|Default|SetCanActivate true)
    ;[0.15 0.15 0.15 0.5] Check if shot or stepped
    (if (or (and (Collision|IsOverlappingActor (Variables|Default|GetCollision) (Variables|Default|GetBP%20First%20Person%20Character) :!class /Script/Engine.PrimitiveComponent) (Variables|Default|GetCanActivate)) (Variables|Default|GetActivated))
      ;[0.15 0.15 0.15 0.5] Activate Plate
      (Rendering|Material|SetScalarParameterValue _dynamic_material "Intensity" 2e+02 :!class /Script/Engine.MaterialInstanceDynamic)
      (Rendering|Material|SetVectorParameterValue _dynamic_material "Colour" "(R=0.000000,G=1.000000,B=0.000000,A=1.000000)" :!class /Script/Engine.MaterialInstanceDynamic)
      (Variables|Default|SetActivated true)
      ;[0.15 0.15 0.15 0.5] Destroy door
      (bind _door (Variables|Default|GetDoor)
        (:then
          (Actor|DestroyActor _door)
          (Variables|Default|SetCanActivate true)
          (Development|PrintString "Door Cleared"))
        (:else)))
    (else
      ;[0.15 0.15 0.15 0.5] Cannot activate
      (Rendering|Material|SetVectorParameterValue (Variables|Default|GetDynamic%20Material) "Colour" "(R=1.000000,G=0.000000,B=0.000000,A=1.000000)" :!class /Script/Engine.MaterialInstanceDynamic))))

(fn ConstructionScript)